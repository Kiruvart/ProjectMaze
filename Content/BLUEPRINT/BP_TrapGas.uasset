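; BP_TrapGas is a gas trap actor that applies damage over time to the player character inside its DamageBox.
; Overlap begin starts a looping timer that passes DOTDamage to the character's HealthUpdate, and overlap end clears it.
; On BeginPlay it caches the player character and binds to its trap event, destroying itself when the broadcast trap type matches its own.
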(event `self.ReceiveBeginPlay`
  (bind _asbp_third_person_character (cast `/Game/ThirdPerson/Blueprints/BP_ThirdPersonCharacter` (`GameplayStatics.GetPlayerCharacter` 0)))
  (bind _output_get (set `self.As BP Third Person Character` _asbp_third_person_character))
  (add `/Game/ThirdPerson/Blueprints/BP_ThirdPersonCharacter.DP_trap` _output_get (delegate `hi :)`)))

(event `hi :)`
  (params (`trap type` :type "/Game/BLUEPRINT/TrapType Enum" :default "NewEnumerator0"))
  (if (`|EnumEquality` `trap type` (`self.Trap Type`))
    (`self.K2_DestroyActor`)))

(event `self.damage box.OnComponentBeginOverlap`
  (params (OverlappedComponent :type "PrimitiveComponent Object Reference") (OtherActor :type "Actor Object Reference") (OtherComp :type "PrimitiveComponent Object Reference") (OtherBodyIndex :type Integer) (bFromSweep :type Boolean) (SweepResult :type "HitResult Structure (by ref)"))
  (if (== OtherActor (`self.As BP Third Person Character`))
    (bind _returnvalue (`KismetSystemLibrary.K2_SetTimerDelegate` (delegate `DOT`) (`self.DOT_time`) true))
    (set `self.NewVar` _returnvalue)))

(event `DOT`
  (`/Game/ThirdPerson/Blueprints/BP_ThirdPersonCharacter.HealthUpdate` (`self.As BP Third Person Character`) (`self.DOT_damage`)))

(event `self.damage box.OnComponentEndOverlap`
  (params (OverlappedComponent :type "PrimitiveComponent Object Reference") (OtherActor :type "Actor Object Reference") (OtherComp :type "PrimitiveComponent Object Reference") (OtherBodyIndex :type Integer))
  (if (== OtherActor (`self.As BP Third Person Character`))
    (`KismetSystemLibrary.K2_ClearAndInvalidateTimerHandle` (`self.NewVar`))))

(fn `NewFunction`)

(fn `UserConstructionScript`)