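; BP_Finish is the level finish trigger that ends the timed run when something overlaps its box.
; On the first overlap only, it stops the timer held by the Start reference.
; It then turns the light on every BP_Floor green and prints a completion message with elapsed seconds, derived from Start's remaining time.
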(event `self.Box.OnComponentBeginOverlap`
  (params (OverlappedComponent :type "PrimitiveComponent Object Reference") (OtherActor :type "Actor Object Reference") (OtherComp :type "PrimitiveComponent Object Reference") (OtherBodyIndex :type Integer) (bFromSweep :type Boolean) (SweepResult :type "HitResult Structure (by ref)"))
  (bind _start (`self.Start`))
  (`/Engine/EditorBlueprintResources/StandardMacros.DoOnce` false
    (:`Completed`
      (`KismetSystemLibrary.K2_ClearAndInvalidateTimerHandle` (`/Game/BLUEPRINT/BP_Start.TimerHandler` _start))
      (bind _outactors (`GameplayStatics.GetAllActorsOfClass` "/Game/BLUEPRINT/BP_Floor.BP_Floor_C"))
      (for _array_element _outactors
        (bind _light (`/Game/BLUEPRINT/BP_Floor.Light` _array_element))
        (`/Engine/EditorBlueprintResources/StandardMacros.IsValid` _light
          (:`Is Valid`
            (`LightComponent.SetLightColor` _light (struct :`R` 0.112749 :`G` 1.0 :`B` 0.025833 :`A` 1.0) true))))
      (`KismetSystemLibrary.PrintString` (`KismetStringLibrary.Concat_StrStr` "well done!" (`KismetStringLibrary.Conv_DoubleToString` (- 30.0 (`/Game/BLUEPRINT/BP_Start.Time` _start))) " SECONDS")))))

(fn `UserConstructionScript`)