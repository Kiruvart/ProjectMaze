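; BP_Spike is a spike trap that moves and hurts the player character.
; Entering the TL trigger restarts a timeline that drives the Trap component's relative Z location, while overlapping the Damage component reduces health through HealthUpdate.
; On BeginPlay it caches the player and binds to their DPTrap event, destroying itself when the broadcast TrapType matches its own.
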(event `self.ReceiveBeginPlay`
  (bind _asbp_third_person_character (cast `/Game/ThirdPerson/Blueprints/BP_ThirdPersonCharacter` (`GameplayStatics.GetPlayerCharacter` 0)))
  (bind _output_get (set `self.As BP Third Person Character` _asbp_third_person_character))
  (add `/Game/ThirdPerson/Blueprints/BP_ThirdPersonCharacter.DP_trap` _output_get (delegate `hi :)`)))

(event `hi :)`
  (params (`trap type` :type "/Game/BLUEPRINT/TrapType Enum" :default "NewEnumerator0"))
  (if (`|EnumEquality` `trap type` (`self.Trap Type`))
    (`self.K2_DestroyActor`)))

(event `self.Damage.OnComponentBeginOverlap`
  (params (OverlappedComponent :type "PrimitiveComponent Object Reference") (OtherActor :type "Actor Object Reference") (OtherComp :type "PrimitiveComponent Object Reference") (OtherBodyIndex :type Integer) (bFromSweep :type Boolean) (SweepResult :type "HitResult Structure (by ref)"))
  (if (== OtherActor (`self.As BP Third Person Character`))
    (`/Game/ThirdPerson/Blueprints/BP_ThirdPersonCharacter.HealthUpdate` (`self.As BP Third Person Character`) -15.0)))

(event `self.TL.OnComponentBeginOverlap`
  (params (OverlappedComponent :type "PrimitiveComponent Object Reference") (OtherActor :type "Actor Object Reference") (OtherComp :type "PrimitiveComponent Object Reference") (OtherBodyIndex :type Integer) (bFromSweep :type Boolean) (SweepResult :type "HitResult Structure (by ref)"))
  (if (== OtherActor (`self.As BP Third Person Character`))
    (bind (_direction _newtrack_0) (`Timeline|Timeline` :!via `PlayFromStart`)
      (:`Update`
        (`SceneComponent.K2_SetRelativeLocation` (`self.trap`) (`KismetMathLibrary.MakeVector` 0.0 0.0 _newtrack_0) false false)))))

(fn `UserConstructionScript`)