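; BP_door is a locked door that swings open and closed on interaction once the key is found.
; The Interract event checks KeyFound and prints a prompt to get the key if it is false.
; Otherwise it flips InteractState and plays or reverses a Timeline, whose track drives a rotator lerp on the Door's relative rotation for a quarter-turn swing.
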(event `/Game/BLUEPRINT/BPI_uiinteract.interract`
  (if (`self.KeyFound`)
    (if (`self.Interact State`)
      (set `self.Interact State` false)
      (bind (_direction _newtrack_0) (`Timeline|Timeline` :!via `Reverse` :!label _label)
        (:`Update`
          (`SceneComponent.K2_SetRelativeRotation` (`self.door`) (`KismetMathLibrary.RLerp` (struct) (struct :`Yaw` -90.0) _newtrack_0) false false)))
      (else
        (set `self.Interact State` true)
        (goto _label)))
    (else
      (`KismetSystemLibrary.PrintString` "GET TEH KEY!!"))))

(fn `UserConstructionScript`)