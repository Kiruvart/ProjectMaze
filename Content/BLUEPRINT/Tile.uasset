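; Tile actor that builds its own boundary walls at runtime, likely as a cell in a grid or maze layout.
; On BeginPlay, a sequence checks the North, South, East and West booleans and spawns a Wall actor on each flagged side.
; Each wall's offset and thin, stretched scale derive from the tile's actor scale, with offsets applied along world axes regardless of the tile's rotation.
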(event `self.ReceiveBeginPlay`
  (`|ExecutionSequence`
    (:`then_0`
      (if (`self.North`)
        (`|SpawnActorFromClass` "/Game/BLUEPRINT/Wall.Wall_C" (`KismetMathLibrary.MakeTransform` (+ (`self.K2_GetActorLocation`) (* (`self.GetActorScale3D`) (250.0 0.0 0.0))) (struct) (* (`self.GetActorScale3D`) (0.1 5.0 5.0))) "Undefined" "MultiplyWithRoot" null null)))
    (:`then_1`
      (if (`self.South`)
        (`|SpawnActorFromClass` "/Game/BLUEPRINT/Wall.Wall_C" (`KismetMathLibrary.MakeTransform` (+ (`self.K2_GetActorLocation`) (* (`self.GetActorScale3D`) (-250.0 0.0 0.0))) (struct) (* (`self.GetActorScale3D`) (0.1 5.0 5.0))) "Undefined" "MultiplyWithRoot" null null)))
    (:`then_2`
      (if (`self.West`)
        (`|SpawnActorFromClass` "/Game/BLUEPRINT/Wall.Wall_C" (`KismetMathLibrary.MakeTransform` (+ (`self.K2_GetActorLocation`) (* (`self.GetActorScale3D`) (0.0 -250.0 0.0))) (struct) (* (`self.GetActorScale3D`) (5.0 0.1 5.0))) "Undefined" "MultiplyWithRoot" null null)))
    (:`then_3`
      (if (`self.East`)
        (`|SpawnActorFromClass` "/Game/BLUEPRINT/Wall.Wall_C" (`KismetMathLibrary.MakeTransform` (+ (`self.K2_GetActorLocation`) (* (`self.GetActorScale3D`) (0.0 250.0 0.0))) (struct) (* (`self.GetActorScale3D`) (5.0 0.1 5.0))) "Undefined" "MultiplyWithRoot" null null)))))

(fn `UserConstructionScript`)