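; BP_Start is a trigger actor that starts a countdown which the player loses when it runs out.
; The first overlap with its Box starts a one-second looping timer event that decrements the Time variable.
; When the count passes zero, it clears the timer, turns the Light on every BP_Floor actor red and prints a losing message.
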(event `self.Box.OnComponentBeginOverlap`
  (params (OverlappedComponent :type "PrimitiveComponent Object Reference") (OtherActor :type "Actor Object Reference") (OtherComp :type "PrimitiveComponent Object Reference") (OtherBodyIndex :type Integer) (bFromSweep :type Boolean) (SweepResult :type "HitResult Structure (by ref)"))
  (`/Engine/EditorBlueprintResources/StandardMacros.DoOnce` false
    (:`Completed`
      (bind _returnvalue (`KismetSystemLibrary.K2_SetTimerDelegate` (delegate `Timer`) 1.0 true))
      (bind _output_get (set `self.TimerHandler` _returnvalue)))))

(event `Timer`
  (bind _result (`/Engine/EditorBlueprintResources/StandardMacros.DecrementFloat` (`self.Time`))
    (:`  `
      (if (< _result 0.0)
        (`KismetSystemLibrary.K2_ClearAndInvalidateTimerHandle` (stale `self.Box.OnComponentBeginOverlap` _output_get))
        (bind _outactors (`GameplayStatics.GetAllActorsOfClass` "/Game/BLUEPRINT/BP_Floor.BP_Floor_C"))
        (for _array_element _outactors
          (`LightComponent.SetLightColor` (`/Game/BLUEPRINT/BP_Floor.Light` _array_element) (struct :`R` 1.0 :`A` 1.0) true))
        (`KismetSystemLibrary.PrintString` "you lost :(")))))

(fn `UserConstructionScript`)