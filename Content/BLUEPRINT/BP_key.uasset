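; BP_key is a key pickup that unlocks a linked Door actor.
; Its Interract event sets KeyFound on the Door, then destroys the key.
; The construction script uses the Color enum to apply one shared material to both the key mesh and the Door's mesh, visually pairing them.
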(event `/Game/BLUEPRINT/BPI_uiinteract.interract`
  (set `/Game/BLUEPRINT/BP_door.KeyFound` true (`self.Door`))
  (`self.K2_DestroyActor`))

(fn `UserConstructionScript`
  (bind _staticmesh (`self.StaticMesh`))
  (switch `|SwitchEnum` (`self.Color`)
    (:`NewEnumerator0`
      (`PrimitiveComponent.SetMaterial` _staticmesh 0 "/Game/LevelPrototyping/Materials/MI_Solid_Blue.MI_Solid_Blue")
      (`PrimitiveComponent.SetMaterial` (`/Game/BLUEPRINT/BP_door.StaticMesh` (`self.Door`)) 0 "/Game/LevelPrototyping/Materials/MI_Solid_Blue.MI_Solid_Blue"))
    (:`NewEnumerator1`
      (`PrimitiveComponent.SetMaterial` _staticmesh 0 "/Game/StarterContent/Materials/M_Metal_Copper.M_Metal_Copper")
      (`PrimitiveComponent.SetMaterial` (`/Game/BLUEPRINT/BP_door.StaticMesh` (`self.Door`)) 0 "/Game/StarterContent/Materials/M_Metal_Copper.M_Metal_Copper"))
    (:`NewEnumerator2`
      (`PrimitiveComponent.SetMaterial` _staticmesh 0 "/Game/StarterContent/Materials/M_Water_Ocean.M_Water_Ocean")
      (`PrimitiveComponent.SetMaterial` (`/Game/BLUEPRINT/BP_door.StaticMesh` (`self.Door`)) 0 "/Game/StarterContent/Materials/M_Water_Ocean.M_Water_Ocean"))))