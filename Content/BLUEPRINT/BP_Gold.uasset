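; BP_Gold is an interactable gold pickup that holds a random amount of gold.
; On BeginPlay it rolls the amount and spawns one to three gold cone meshes, with larger amounts showing more cones, each placed at the relative transform of a preset component.
; Interacting adds the amount to the player character's Gold, refreshes its text and destroys the pickup.
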(event `/Game/BLUEPRINT/BPI_uiinteract.interract`
  (bind _asbp_third_person_character (cast `/Game/ThirdPerson/Blueprints/BP_ThirdPersonCharacter` (`GameplayStatics.GetPlayerCharacter` 0)))
  (set `/Game/ThirdPerson/Blueprints/BP_ThirdPersonCharacter.Gold` (+ (`/Game/ThirdPerson/Blueprints/BP_ThirdPersonCharacter.Gold` _asbp_third_person_character) (`self.GoldAmount`)) _asbp_third_person_character)
  (`/Game/ThirdPerson/Blueprints/BP_ThirdPersonCharacter.RefreshText` _asbp_third_person_character)
  (`self.K2_DestroyActor`))

(event `self.ReceiveBeginPlay`
  (set `self.GoldAmount` (`KismetMathLibrary.RandomIntegerInRange` 1 99))
  (bind _returnvalue (`AddComponent|NODE_AddStaticMeshComponent-0` :`RelativeTransform` (`SceneComponent.GetRelativeTransform` (`self.1`))))
  (`StaticMeshComponent.SetStaticMesh` _returnvalue "/Game/StarterContent/Shapes/Shape_Cone.Shape_Cone")
  (`PrimitiveComponent.SetMaterial` _returnvalue 0 "/Game/StarterContent/Materials/M_Metal_Gold.M_Metal_Gold")
  (if (>= (`self.GoldAmount`) 26)
    (bind _returnvalue_2 (`AddComponent|NODE_AddStaticMeshComponent-1` :`RelativeTransform` (`SceneComponent.GetRelativeTransform` (`self.2`))))
    (`StaticMeshComponent.SetStaticMesh` _returnvalue_2 "/Game/StarterContent/Shapes/Shape_Cone.Shape_Cone")
    (`PrimitiveComponent.SetMaterial` _returnvalue_2 0 "/Game/StarterContent/Materials/M_Metal_Gold.M_Metal_Gold")
    (if (>= (`self.GoldAmount`) 76)
      (bind _returnvalue_3 (`AddComponent|NODE_AddStaticMeshComponent-2` :`RelativeTransform` (`SceneComponent.GetRelativeTransform` (`self.3`))))
      (`StaticMeshComponent.SetStaticMesh` _returnvalue_3 "/Game/StarterContent/Shapes/Shape_Cone.Shape_Cone")
      (`PrimitiveComponent.SetMaterial` _returnvalue_3 0 "/Game/StarterContent/Materials/M_Metal_Gold.M_Metal_Gold"))))

(fn `UserConstructionScript`)