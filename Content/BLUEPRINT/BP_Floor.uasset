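; BP_Floor is a modular grid-cell room piece that builds a floor with optional walls, ceiling and light.
; The Construction Script scales the floor cube to GridSize and derives wall thickness from it.
; Direction and Ceiling flags add offset static mesh components, sized through the CubeScale helper from world dimensions.
; A positive IntensityLight adds a colored point light centered near the top; the event graph holds no logic.
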(fn `UserConstructionScript`
  (locals (`Wall Thickness` :type "Float (double-precision)") (`Wall Lenght` :type "Float (double-precision)"))
  (bind _grid_size (`self.Grid Size`))
  (bind _wall_lenght (`local.Wall Lenght`))
  (bind _wall_lenght_2 (`local.Wall Lenght`))
  (bind _returnvalue (* (`local.Wall Lenght`) 0.5))
  (set `local.Wall Lenght` _grid_size)
  (set `local.Wall Thickness` (* _grid_size 0.1))
  (`SceneComponent.SetRelativeScale3D` (`self.Cube`) (`self.Cube Scale` (`KismetMathLibrary.MakeVector` _wall_lenght_2 _wall_lenght_2 (`local.Wall Thickness`))))
  (`|ExecutionSequence`
    (:`then_0`
      (if (`self.West`)
        (`AddComponent|NODE_AddStaticMeshComponent-0` :`RelativeTransform` (`KismetMathLibrary.MakeTransform` (0.0 0.0 0.0) (struct) (`self.Cube Scale` (`KismetMathLibrary.MakeVector` (`local.Wall Lenght`) (`local.Wall Thickness`) (`self.Wall Height`)))))))
    (:`then_1`
      (if (`self.South`)
        (`AddComponent|NODE_AddStaticMeshComponent-1` :`RelativeTransform` (`KismetMathLibrary.MakeTransform` (0.0 0.0 0.0) (struct) (`self.Cube Scale` (`KismetMathLibrary.MakeVector` (`local.Wall Thickness`) (`local.Wall Lenght`) (`self.Wall Height`)))))))
    (:`then_2`
      (if (`self.North`)
        (`AddComponent|NODE_AddStaticMeshComponent-2` :`RelativeTransform` (`KismetMathLibrary.MakeTransform` (`KismetMathLibrary.MakeVector` (- (`local.Wall Lenght`) (`local.Wall Thickness`))) (struct) (`self.Cube Scale` (`KismetMathLibrary.MakeVector` (`local.Wall Thickness`) (`local.Wall Lenght`) (`self.Wall Height`)))))))
    (:`then_3`
      (if (`self.East`)
        (`AddComponent|NODE_AddStaticMeshComponent-3` :`RelativeTransform` (`KismetMathLibrary.MakeTransform` (`KismetMathLibrary.MakeVector` 0.0 (- (`local.Wall Lenght`) (`local.Wall Thickness`))) (struct) (`self.Cube Scale` (`KismetMathLibrary.MakeVector` (`local.Wall Lenght`) (`local.Wall Thickness`) (`self.Wall Height`)))))))
    (:`then_4`
      (if (`self.Ceiling`)
        (`AddComponent|NODE_AddStaticMeshComponent-5` :`RelativeTransform` (`KismetMathLibrary.MakeTransform` (`KismetMathLibrary.MakeVector` 0.0 0.0 (`self.Wall Height`)) (struct) (`self.Cube Scale` (`KismetMathLibrary.MakeVector` _wall_lenght _wall_lenght (`local.Wall Thickness`)))))))
    (:`then_5`
      (if (> (`self.Intensity Light`) 0.0)
        (bind _returnvalue_2 (`AddComponent|NODE_AddPointLightComponent-0` :`RelativeTransform` (`KismetMathLibrary.MakeTransform` (`KismetMathLibrary.MakeVector` _returnvalue _returnvalue (* (`self.Wall Height`) 0.9)))))
        (set `self.Light` _returnvalue_2)
        (`LightComponent.SetLightColor` _returnvalue_2 (`self.Color Light`) true)
        (`LightComponent.SetIntensity` _returnvalue_2 (`self.Intensity Light`))))))